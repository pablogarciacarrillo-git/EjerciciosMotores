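; BordeX is a map border actor that fades into view as the player character approaches it along the X axis.
; The construction script creates a dynamic instance of the border material on its static mesh, and BeginPlay caches the MyCharacter actor.
; Each Tick sets the material's Opacity from the X distance to the character, rising linearly within a fixed range and staying invisible beyond it.
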(event `self.ReceiveBeginPlay`
  (bind _returnvalue (`GameplayStatics.GetActorOfClass` "/Game/Dynamic/Character/MyCharacter.MyCharacter_C"))
  (set `self.Character` _returnvalue))

(event `self.ReceiveTick`
  (params (DeltaSeconds :type "Float (single-precision)"))
  (bind _returnvalue_x (`KismetMathLibrary.BreakVector` (`self.K2_GetActorLocation`)))
  (bind _bordematerial (`self.BordeMaterial`))
  (bind _returnvalue_x_2 (`KismetMathLibrary.BreakVector` (`self.K2_GetActorLocation` (`self.Character`))))
  (bind _returnvalue (`KismetMathLibrary.Abs` (- _returnvalue_x_2 _returnvalue_x)))
  (if (<= _returnvalue 500.0)
    (`MaterialInstanceDynamic.SetScalarParameterValue` _bordematerial "Opacity" (- 1.0 (/ _returnvalue 500.0)))
    (else
      (`MaterialInstanceDynamic.SetScalarParameterValue` _bordematerial "Opacity" 0.0))))

(fn `UserConstructionScript`
  (bind _returnvalue (`PrimitiveComponent.CreateDynamicMaterialInstance` (`self.StaticMeshComponent`) 0 "/Game/Dynamic/Materials/BordesMapaMaterial.BordesMapaMaterial" "None"))
  (set `self.BordeMaterial` _returnvalue))