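; Behavior tree task that makes an AI, labeled a turret in its logs, flee from the player.
; On execute it moves the controller toward a point three units along the normalized direction away from player pawn 0, using the controller's own location as the origin.
; It only logs progress and never calls Finish Execute.
; The log labeled as player position prints the controller's location.
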(event `self.ReceiveExecuteAI`
  (params (OwnerController :type "AIController Object Reference") (ControlledPawn :type "Pawn Object Reference"))
  (bind _returnvalue (`Actor.K2_GetActorLocation` OwnerController))
  (bind _returnvalue_2 (`KismetStringLibrary.Conv_VectorToString` _returnvalue))
  (`AITask_MoveTo.AIMoveTo` OwnerController (+ (* (`KismetMathLibrary.Normal` (- _returnvalue (`Actor.K2_GetActorLocation` (`GameplayStatics.GetPlayerPawn` 0)))) 3) _returnvalue) null -1.0 "Default" "Default" true false
    (:`then`
      (`KismetSystemLibrary.LogString` (`KismetStringLibrary.Concat_StrStr` "Posicion Torreta: " _returnvalue_2))
      (`KismetSystemLibrary.LogString` (`KismetStringLibrary.Concat_StrStr` "Posicion Player: " _returnvalue_2)))
    (:`OnRequestFailed`
      (`KismetSystemLibrary.LogString` "Flee Fallido"))
    (:`OnMoveFinished`
      (`KismetSystemLibrary.LogString` "Flee Finalizado"))))