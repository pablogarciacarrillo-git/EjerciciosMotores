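; Turret actor that aims at the player and fires bullets while MyCharacter is within ShootRange.
; BeginPlay caches the first MyCharacter and starts a looping timer with a random 3 to 10 second interval, rolled once.
; Each timer tick spawns a Bullet at the ShootPoint transform if the character is in range.
; Tick turns the Head toward player pawn 0 under the same range check.
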(event `self.ReceiveBeginPlay`
  (bind _returnvalue (`GameplayStatics.GetActorOfClass` "/Game/Dynamic/Character/MyCharacter.MyCharacter_C"))
  (set `self.Character` _returnvalue)
  (`KismetSystemLibrary.K2_SetTimerDelegate` (delegate `CustomEvent`) (`KismetMathLibrary.RandomFloatInRange` 3.0 10.0) true))

(event `CustomEvent`
  (if (< (`self.GetDistanceTo` (`self.Character`)) (`self.ShootRange`))
    (`self.Shoot`)))

(event `self.ReceiveTick`
  (params (DeltaSeconds :type "Float (single-precision)"))
  (if (< (`self.GetDistanceTo` (`self.Character`)) (`self.ShootRange`))
    (`SceneComponent.K2_SetWorldRotation` (`self.Head`) (`KismetMathLibrary.FindLookAtRotation` (`SceneComponent.K2_GetComponentLocation` (`self.Head`)) (`self.K2_GetActorLocation` (`GameplayStatics.GetPlayerPawn` 0))) false false)))

(fn `Shoot`
  (`|SpawnActorFromClass` "/Game/Dynamic/Blueprints/Bullet.Bullet_C" (`SceneComponent.K2_GetComponentToWorld` (`self.ShootPoint`)) "Undefined" "MultiplyWithRoot" null null))

(fn `UserConstructionScript`)