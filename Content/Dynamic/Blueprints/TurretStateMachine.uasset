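; Turret enemy that targets MyCharacter, tracking it with its head and shooting when it is within detection distance.
; BeginPlay gives the Blackboard the target and waypoint and starts a looping fire timer whose interval is randomized once, spawning bullets at ShootPoint.
; Tick updates target distance and a flee point directly away from the player in the Blackboard, aims the head, and plays a one-time activation sound on first detection.
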(event `self.ReceiveBeginPlay`
  (bind _returnvalue (`AIBlueprintHelperLibrary.GetBlackboard` null))
  (bind _returnvalue_2 (`GameplayStatics.GetActorOfClass` "/Game/Dynamic/Character/MyCharacter.MyCharacter_C"))
  (bind _output_get (set `self.Target` _returnvalue_2))
  (`BlackboardComponent.SetValueAsObject` _returnvalue (`KismetStringLibrary.Conv_StringToName` "Target") _output_get)
  (`BlackboardComponent.SetValueAsObject` _returnvalue (`KismetStringLibrary.Conv_StringToName` "Waypoint") (`self.Waypoint`))
  (`KismetSystemLibrary.K2_SetTimerDelegate` (delegate `CustomEvent`) (`KismetMathLibrary.RandomFloatInRange` 3.0 10.0) true))

(event `self.ReceiveTick`
  (params (DeltaSeconds :type "Float (single-precision)"))
  (bind _returnvalue (`self.K2_GetActorLocation`))
  (bind _returnvalue_2 (`AIBlueprintHelperLibrary.GetBlackboard` null))
  (bind _head (`self.Head`))
  (bind _returnvalue_3 (`self.GetDistanceTo` (`self.Target`)))
  (bind _returnvalue_4 (`SceneComponent.K2_GetComponentLocation` _head))
  (`BlackboardComponent.SetValueAsVector` _returnvalue_2 (`KismetStringLibrary.Conv_StringToName` "FleeTarget") (`KismetMathLibrary.MakeVector` (.x (+ _returnvalue (* (`KismetMathLibrary.GetForwardVector` (`KismetMathLibrary.FindLookAtRotation` _returnvalue (`self.K2_GetActorLocation` (`self.Target`)))) -500.0))) (.y (+ _returnvalue (* (`KismetMathLibrary.GetForwardVector` (`KismetMathLibrary.FindLookAtRotation` _returnvalue (`self.K2_GetActorLocation` (`self.Target`)))) -500.0))) (.z _returnvalue)))
  (`BlackboardComponent.SetValueAsFloat` _returnvalue_2 (`KismetStringLibrary.Conv_StringToName` "DistanceToTarget") _returnvalue_3)
  (if (< _returnvalue_3 (`self.DetectionDistance`))
    (`SceneComponent.K2_SetWorldRotation` _head (`KismetMathLibrary.FindLookAtRotation` _returnvalue_4 (`self.K2_GetActorLocation` (`self.Target`))) false false)
    (`/Engine/EditorBlueprintResources/StandardMacros.DoOnce` false
      (:`Completed`
        (`GameplayStatics.PlaySoundAtLocation` "/Game/Dynamic/Sounds/Turret/TurretActivation.TurretActivation" _returnvalue_4 (struct) 1.0 1.0 0.0 null null null null)))))

(event `CustomEvent`
  (if (< (`self.GetDistanceTo` (`self.Target`)) (`self.DetectionDistance`))
    (`self.Shoot`)))

(fn `Shoot`
  (`|SpawnActorFromClass` "/Game/Dynamic/Blueprints/Bullet.Bullet_C" (`SceneComponent.K2_GetComponentToWorld` (`self.ShootPoint`)) "Undefined" "MultiplyWithRoot" null null))

(fn `UserConstructionScript`)